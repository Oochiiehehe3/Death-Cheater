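; Street knife actor that detects hits on actors carrying a Health component.
; On a mesh hit it calls TakeDmg on that component with zero damage, then prints a scaled speed value from the attach parent actor's velocity.
; That speed does not feed the damage, and a minimum-speed check is left disconnected.
; Tick prints a component velocity from the mesh's attach hierarchy every frame for debugging.
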(event OnComponentHit(StaticMeshComponent)
  (params (HitComponent :type Primitive%20Component%20Object%20Reference) (OtherActor :type Actor%20Object%20Reference) (OtherComp :type Primitive%20Component%20Object%20Reference) (NormalImpulse :type Vector :default "0, 0, 0") (Hit :type Hit%20Result%20Structure%20%28by%20ref%29))
  (bind _returnvalue (Actor|GetComponentsByClass OtherActor "/Game/Blueprints/health.health_C"))
  (bind _returnvalue_2 (Actor|GetAttachParentActor))
  (bind _returnvalue_3 (Transformation|GetVelocity _returnvalue_2))
  (if (Utilities|Array|IsNotEmpty _returnvalue)
    (Default|TakeDmg (Utilities|Select :Index 0 :Option%200 _returnvalue :Option%201 0))
    (Development|PrintString (Utilities|String|ToString(Integer) (Math|Float|Truncate (/ (+ (Math|Float|Absolute(Float) (.x _returnvalue_3)) (Math|Float|Absolute(Float) (.y _returnvalue_3)) (Math|Float|Absolute(Float) (.z _returnvalue_3))) 1e+03))) true true "(R=0.473150,G=0.000000,B=1.000000,A=1.000000)" 1e+02)))

(event EventBeginPlay)

(event Collision|EventActorBeginOverlap
  (params (OtherActor :type Actor%20Object%20Reference)))

(event EventTick
  (params (DeltaSeconds :type Float%20%28single-precision%29))
  (Development|PrintString (Utilities|String|ToString(Vector) (Transformation|GetComponentVelocity (Components|GetChildComponent (Transformation|GetAttachParent (Variables|Debug|GetStaticMeshComponent)) 0)))))

(fn ConstructionScript)