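; Health component that tracks its owning actor's hit points and destroys that actor when they run out.
; TakeDmg subtracts damage from ObjHealth, or on a lethal hit teleports the owner far away along negative Y and starts a short timer.
; The timer calls Death by name to destroy the owner, so the actor is relocated briefly before removal.
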(event EventBeginPlay)

(event EventTick
  (params (DeltaSeconds :type Float%20%28single-precision%29)))

(fn TakeDmg
  (params (dmg :type Integer))
  (if (<= (- (Variables|Default|Getobj_health) dmg) 0)
    (Transformation|SetActorLocation (Components|GetOwner) "0.000000,-10000.000000,0.000000" false false)
    (Utilities|Time|SetTimerbyFunctionName 0 "death" 0.1)
    (else
      (Variables|Default|Setobj_health (- (Variables|Default|Getobj_health) dmg)))))

(fn Death
  (Actor|DestroyActor (Components|GetOwner)))