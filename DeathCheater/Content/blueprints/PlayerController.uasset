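; A VR player controller that moves its pawn with physics forces on the capsule, handling smooth movement, dash and jump input.
; SmoothMove pushes the capsule along stick input rotated by the headset's orientation while summed horizontal speed stays under a cap, printing that speed for debugging.
; Dash applies force scaled from current velocity, then a half-strength counter-force after a one-second lockout.
; Jump adds an upward impulse unless the pawn is falling.
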(event Input|EnhancedActionEvents|EnhancedInputActionSmoothMove
  (params (ActionValue :type Vector%202D%20Structure) (ElapsedSeconds :type Float%20%28double-precision%29) (TriggeredSeconds :type Float%20%28double-precision%29) (InputAction :type Input%20Action%20Object%20Reference :default "/Game/VRTemplate/Input/Actions/SmoothMove.SmoothMove"))
  (bind _returnvalue (Pawn|GetControlledPawn))
  (bind _returnvalue_2 (Actor|GetComponentbyClass _returnvalue "/Script/Engine.CapsuleComponent"))
  (bind _returnvalue_3 (Transformation|GetWorldTransform _returnvalue_2))
  (bind _returnvalue_4 (Transformation|GetComponentVelocity _returnvalue_2))
  (bind _returnvalue_5 (Math|Float|Absolute(Float) (.x _returnvalue_4)))
  (bind _returnvalue_6 (Math|Float|Absolute(Float) (.y _returnvalue_4)))
  (bind _returnvalue_7 (+ _returnvalue_5 _returnvalue_6))
  (Development|PrintString (Utilities|String|ToString(Float) _returnvalue_7))
  (if (<= _returnvalue_7 1e+03)
    (Physics|AddForce _returnvalue_2 (* (* (Math|Transform|TransformDirection (Math|Transform|MakeTransform (.location _returnvalue_3) (.DeviceRotation (Class|HeadMountedDisplayFunctionLibrary|GetOrientationandPosition)) (.scale _returnvalue_3)) (Math|Vector|MakeVector (.y ActionValue) (.x ActionValue) 0.0)) 2e+03) 1) "None" true)))

(event Input|EnhancedActionEvents|EnhancedInputActionDash
  (params (ActionValue :type Boolean) (ElapsedSeconds :type Float%20%28double-precision%29) (TriggeredSeconds :type Float%20%28double-precision%29) (InputAction :type Input%20Action%20Object%20Reference :default "/Game/VRTemplate/Input/Actions/Dash.Dash"))
  (bind _returnvalue (Pawn|GetControlledPawn))
  (bind _returnvalue_2 (Actor|GetComponentbyClass _returnvalue "/Script/Engine.CapsuleComponent"))
  (if (not (Variables|Default|GetisDashing))
    (Variables|Default|SetisDashing true)
    (bind _output_get (Variables|Default|Setbefore%20dash (* (Transformation|GetComponentVelocity _returnvalue_2) 100)))
    (Physics|AddForce _returnvalue_2 (Math|Vector|MakeVector (.x _output_get) (.y _output_get) 0.0) "None" true)
    (Utilities|FlowControl|Delay 1.0)
    (Variables|Default|SetisDashing false)
    (Physics|AddForce _returnvalue_2 (Math|Vector|MakeVector (* (.x (Variables|Default|Getbefore%20dash)) -0.5) (* (.y (Variables|Default|Getbefore%20dash)) -0.5) 0.0) "None" true)))

(event Input|ActionEvents|InputActionJump
  (params (Key :type Key%20Structure :default "None"))
  (:Pressed
    (if (not (AI|Components|NavMovement|IsFalling (Pawn|GetMovementComponent (Pawn|GetControlledPawn))))
      (Physics|AddImpulse (Actor|GetComponentbyClass (Pawn|GetControlledPawn) "/Script/Engine.CapsuleComponent") (Math|Vector|MakeVector 0.0 0.0 2e+01) "None" false))))

(fn ConstructionScript)