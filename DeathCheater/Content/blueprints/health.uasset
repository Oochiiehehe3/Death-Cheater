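; Health component that gives its owning actor damageable health and rewards the player with health for damaging or destroying it.
; TakeDmg subtracts damage from ObjHealth and raises the VR pawn's Playerhealth by the damage plus a bonus.
; A lethal hit grants a fixed bonus instead, moves the owner far below the origin and starts a short timer that calls Death to destroy it.
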(event EventBeginPlay)

(event EventTick
  (params (DeltaSeconds :type Float%20%28single-precision%29)))

(fn TakeDmg
  (params (dmg :type Integer))
  (bind _asvrpawn (Utilities|Casting|CastToVRPawn (Game|Player|GetPlayerPawn 0)))
  (if (<= (- (Variables|Default|Getobj_health) dmg) 0)
    (Transformation|SetActorLocation (Components|GetOwner) "0.000000,-10000.000000,0.000000" false false)
    (Utilities|Time|SetTimerbyFunctionName 0 "death" 0.1)
    (Variables|/Game/VRTemplate/Blueprints/VRPawn.VRPawn_C|Setplayerhealth _asvrpawn (+ 45.0 (Variables|/Game/VRTemplate/Blueprints/VRPawn.VRPawn_C|Getplayerhealth _asvrpawn)))
    (else
      (Variables|Default|Setobj_health (- (Variables|Default|Getobj_health) dmg))
      (Variables|/Game/VRTemplate/Blueprints/VRPawn.VRPawn_C|Setplayerhealth _asvrpawn (+ (+ (Variables|/Game/VRTemplate/Blueprints/VRPawn.VRPawn_C|Getplayerhealth _asvrpawn) dmg) 15.0)))))

(fn Death
  (Actor|DestroyActor (Components|GetOwner)))