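; Street knife Blueprint that damages overlapped actors with a Health component based on how fast it moves.
; Tick uses a FlipFlop to sample the mesh's world position every other frame, storing the delta as velocity.
; On overlap, a sufficiently fast swing calls TakeDmg with clamped, truncated speed and prints it.
; LastComponentsHit blocks repeat hits until overlap ends, and its length toggles Spark visibility.
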(event OnComponentHit(StaticMeshComponent)
  (params (HitComponent :type Primitive%20Component%20Object%20Reference) (OtherActor :type Actor%20Object%20Reference) (OtherComp :type Primitive%20Component%20Object%20Reference) (NormalImpulse :type Vector :default "0, 0, 0") (Hit :type Hit%20Result%20Structure%20%28by%20ref%29)))

(event OnComponentEndOverlap(StaticMeshComponent)
  (params (OverlappedComponent :type Primitive%20Component%20Object%20Reference) (OtherActor :type Actor%20Object%20Reference) (OtherComp :type Primitive%20Component%20Object%20Reference) (OtherBodyIndex :type Integer))
  (Utilities|Array|RemoveItem (Variables|Default|Getlast_components_hit) OtherActor))

(event OnComponentBeginOverlap(StaticMeshComponent)
  (params (OverlappedComponent :type Primitive%20Component%20Object%20Reference) (OtherActor :type Actor%20Object%20Reference) (OtherComp :type Primitive%20Component%20Object%20Reference) (OtherBodyIndex :type Integer) (bFromSweep :type Boolean) (SweepResult :type Hit%20Result%20Structure%20%28by%20ref%29))
  (CallFunction|Dmg OtherActor))

(event Custom|dmg
  (params (other%20actor :type Actor%20Object%20Reference))
  (bind _returnvalue (Actor|GetComponentsByClass other%20actor "/Game/blueprints/health.health_C"))
  (bind _useable_velocity (Variables|Default|Getuseable_velocity))
  (bind _returnvalue_2 (Math|Float|Absolute(Float) (.x _useable_velocity)))
  (bind _returnvalue_3 (Math|Float|Absolute(Float) (.z _useable_velocity)))
  (bind _returnvalue_4 (Math|Float|Absolute(Float) (.y _useable_velocity)))
  (bind _returnvalue_5 (+ _returnvalue_2 _returnvalue_4 _returnvalue_3))
  (bind _returnvalue_6 (Math|Float|Clamp(Float) _returnvalue_5 5.0 25.0))
  (bind _returnvalue_7 (Math|Float|Truncate _returnvalue_6))
  (if (not (Utilities|Array|ContainsItem (Variables|Default|Getlast_components_hit) other%20actor))
    (if (Utilities|Array|IsNotEmpty _returnvalue)
      (Utilities|Array|Insert (Variables|Default|Getlast_components_hit) other%20actor)
      (if (>= _returnvalue_5 2.5)
        (Development|PrintString (Utilities|String|ToString(Integer) _returnvalue_7) true true "(R=0.473150,G=0.000000,B=1.000000,A=1.000000)" 1e+02)
        (Default|TakeDmg (Utilities|Select :Index 0 :Option%200 _returnvalue :Option%201 0) _returnvalue_7)))))

(event EventBeginPlay
  (Collision|SetCollisionResponsetoChannel (Variables|Debug|GetStaticMeshComponent) "ECC_GameTraceChannel2" "ECR_Ignore"))

(event EventTick
  (params (DeltaSeconds :type Float%20%28single-precision%29))
  (Utilities|FlowControl|Sequence
    (:then_0
      (Utilities|FlowControl|FlipFlop
        (:A
          (Variables|Default|Setlast_frame_pos (Variables|Default|Getcurrent_frame_pos))
          (Variables|Default|Setcurrent_frame_pos (Transformation|GetWorldLocation (Variables|Debug|GetStaticMeshComponent)))
          (Variables|Default|Setuseable_velocity (- (Variables|Default|Getcurrent_frame_pos) (Variables|Default|Getlast_frame_pos))))))
    (:then_1
      (if (>= 1 (Utilities|Array|Length (Variables|Default|Getlast_components_hit)))
        (Rendering|SetVisibility (Variables|Default|Getspark) true false)
        (else
          (Rendering|SetVisibility (Variables|Default|Getspark) false false))))))

(fn ConstructionScript)