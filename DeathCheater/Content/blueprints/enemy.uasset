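; Enemy pawn Blueprint that chases the player on sight and wanders in panic during a lockdown.
; PawnSensing sets IsSeeingPlayer, never cleared here, and issues an AIMoveTo toward the player character.
; Until a sighting, Tick starts the panic routine once LockdownHappening is true, guarded by IsPanicing.
; Panic runs to random nearby navigable points, idling briefly and repeating only after successful moves, with animations played directly on the mesh.
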(event OnSeePawn(PawnSensing)
  (params (Pawn :type Pawn%20Object%20Reference))
  ;[1 1 1] Chase
  (Variables|Default|SetisSeeingPlayer true)
  (CallFunction|FollowPlayer))

(event Custom|FollowPlayer
  (bind _returnvalue (Game|GetPlayerCharacter 0))
  ;[1 1 1] Chase
  (if (Variables|Default|GetisSeeingPlayer)
    (AI|AIMoveTo self (Transformation|GetWorldLocation (Actor|GetComponentbyClass _returnvalue "/Script/Engine.CapsuleComponent")) _returnvalue 1.0 true)))

(event Custom|panicmovment
  ;[1 1 1] Panicedmovment
  (Components|Animation|PlayAnimation (Variables|Character|GetMesh) "/Game/Characters/Mannequins/Animations/Manny/MM_Run_Fwd.MM_Run_Fwd" true :!label _label)
  (bind _randomlocation (Class|NavigationSystemV1|GetRandomLocationinNavigableRadius (Transformation|GetActorLocation) 2e+02 0 0))
  (AI|AIMoveTo self _randomlocation 0 5.0 false
    (:OnSuccess
      (Components|Animation|PlayAnimation (Variables|Character|GetMesh) "/Game/Characters/Mannequins/Animations/Manny/MM_Idle.MM_Idle" true)
      (Utilities|FlowControl|Delay 0.2)
      (goto _label))))

(event EventTick
  (params (DeltaSeconds :type Float%20%28single-precision%29))
  ;[1 1 1] Idle
  (if (== (Variables|Default|GetisSeeingPlayer) false)
    (if (== (Variables|Default|GetlockdownHappening) true)
      (if (== (Variables|Default|GetisPanicing) false)
        (Variables|Default|SetisPanicing true)
        (CallFunction|Panicmovment)))))

(fn ConstructionScript)