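; Test human enemy pawn that detects and melees the VR player.
; On sighting a VRPawn, Pawn Sensing writes a seen flag and the target into the AI controller's blackboard.
; The Attack event enables Fist collision for a short timed window, and any VRPawn overlapping the fist loses a fixed amount of health.
; A direct AI move-to-player node is left unconnected.
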(event OnComponentBeginOverlap(Fist)
  (params (OverlappedComponent :type Primitive%20Component%20Object%20Reference) (OtherActor :type Actor%20Object%20Reference) (OtherComp :type Primitive%20Component%20Object%20Reference) (OtherBodyIndex :type Integer) (bFromSweep :type Boolean) (SweepResult :type Hit%20Result%20Structure%20%28by%20ref%29))
  ;[1 1 1] Collison
  (bind _asvrpawn (Utilities|Casting|CastToVRPawn OtherActor))
  (Variables|/Game/VRTemplate/Blueprints/VRPawn.VRPawn_C|Setplayerhealth _asvrpawn (- (Variables|/Game/VRTemplate/Blueprints/VRPawn.VRPawn_C|Getplayerhealth _asvrpawn) 15.0)))

(event OnSeePawn(PawnSensing)
  (params (Pawn :type Pawn%20Object%20Reference))
  (bind _self self)
  (bind _returnvalue (AI|GetAIController _self))
  (bind _returnvalue_2 (AI|GetBlackboard _returnvalue))
  (bind _asvrpawn (Utilities|Casting|CastToVRPawn Pawn))
  (if true
    (AI|Components|Blackboard|SetValueasBool _returnvalue_2 (Utilities|Name|MakeLiteralName "hasSeenPlayer") true)
    (AI|Components|Blackboard|SetValueasObject _returnvalue_2 (Utilities|Name|MakeLiteralName "target") _asvrpawn)))

(event Custom|Attack
  ;[1 1 1] Collison
  (Collision|SetCollisionEnabled (Variables|Default|GetFist) "QueryAndPhysics")
  (Utilities|FlowControl|Delay 1.0)
  (Collision|SetCollisionEnabled (Variables|Default|GetFist) "NoCollision"))

(fn ConstructionScript
  (|CallParentFunction))