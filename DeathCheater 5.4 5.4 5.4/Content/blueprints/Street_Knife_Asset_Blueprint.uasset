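; Street knife weapon that damages any hit actor carrying a Health component, based on how fast the knife is moving.
; Tick uses a FlipFlop to sample the mesh position every other frame, giving a per-sample displacement as velocity.
; Hits above a speed threshold deal that summed axis movement as clamped damage and print it for debugging.
; A gate closes after each hit and reopens when any overlap ends.
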(event OnComponentHit(StaticMeshComponent)
  (params (HitComponent :type Primitive%20Component%20Object%20Reference) (OtherActor :type Actor%20Object%20Reference) (OtherComp :type Primitive%20Component%20Object%20Reference) (NormalImpulse :type Vector :default "0, 0, 0") (Hit :type Hit%20Result%20Structure%20%28by%20ref%29))
  (bind _returnvalue (Actor|GetComponentsByClass OtherActor "/Game/blueprints/health.health_C"))
  (bind _useable_velocity (Variables|Default|Getuseable_velocity))
  (bind _returnvalue_2 (Math|Float|Absolute(Float) (.x _useable_velocity)))
  (bind _returnvalue_3 (Math|Float|Absolute(Float) (.z _useable_velocity)))
  (bind _returnvalue_4 (Math|Float|Absolute(Float) (.y _useable_velocity)))
  (bind _returnvalue_5 (+ _returnvalue_2 _returnvalue_4 _returnvalue_3))
  (bind _returnvalue_6 (Math|Float|Clamp(Float) _returnvalue_5 5.0 25.0))
  (bind _returnvalue_7 (Math|Float|Truncate _returnvalue_6))
  (Utilities|FlowControl|Gate false :!label _label
    (:Exit
      (Utilities|FlowControl|Sequence
        (:then_0
          (if (Utilities|Array|IsNotEmpty _returnvalue)
            (if (>= _returnvalue_5 3.0)
              (Default|TakeDmg (Utilities|Select :Index 0 :Option%200 _returnvalue :Option%201 0) _returnvalue_7)
              (Development|PrintString (Utilities|String|ToString(Integer) _returnvalue_7) true true "(R=0.473150,G=0.000000,B=1.000000,A=1.000000)" 1e+02))))
        (:then_1
          (goto _label Close))))))

(event OnComponentEndOverlap(StaticMeshComponent)
  (params (OverlappedComponent :type Primitive%20Component%20Object%20Reference) (OtherActor :type Actor%20Object%20Reference) (OtherComp :type Primitive%20Component%20Object%20Reference) (OtherBodyIndex :type Integer))
  (bind _useable_velocity (Variables|Default|Getuseable_velocity))
  (bind _returnvalue (Math|Float|Absolute(Float) (.x _useable_velocity)))
  (bind _returnvalue_2 (Math|Float|Absolute(Float) (.z _useable_velocity)))
  (bind _returnvalue_3 (Math|Float|Absolute(Float) (.y _useable_velocity)))
  (bind _returnvalue_4 (+ _returnvalue _returnvalue_3 _returnvalue_2))
  (bind _returnvalue_5 (Math|Float|Clamp(Float) _returnvalue_4 5.0 25.0))
  (bind _returnvalue_6 (Math|Float|Truncate _returnvalue_5))
  (if (== (stale OnComponentHit(StaticMeshComponent) OtherActor) OtherActor)
    (Utilities|FlowControl|Gate false) ; enters at Open
  ))

(event EventBeginPlay)

(event Collision|EventActorBeginOverlap
  (params (OtherActor :type Actor%20Object%20Reference)))

(event EventTick
  (params (DeltaSeconds :type Float%20%28single-precision%29))
  (Utilities|FlowControl|FlipFlop
    (:A
      (Variables|Default|Setlast_frame_pos (Variables|Default|Getcurrent_frame_pos))
      (Variables|Default|Setcurrent_frame_pos (Transformation|GetWorldLocation (Variables|Debug|GetStaticMeshComponent)))
      (Variables|Default|Setuseable_velocity (- (Variables|Default|Getcurrent_frame_pos) (Variables|Default|Getlast_frame_pos))))
    (:B
      (Utilities|FlowControl|DelayUntilNextTick))))

(fn ConstructionScript)